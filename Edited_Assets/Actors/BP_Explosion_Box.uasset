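; BP_Explosion_Box is a hazard actor that damages and knocks back the learning kit player character when it overlaps the Sphere component.
; The overlap subtracts a fixed amount from CurrentHealth, refreshes the health bar widget and sets IsHit.
; The launch flattens and normalizes the sphere-to-player direction, adds a unit upward component, scales by LaunchVelocity and overrides current velocity.
; It contains no explosion effect or self-destruction logic.
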(event `self.Sphere.OnComponentBeginOverlap`
  (params (OverlappedComponent :type "PrimitiveComponent Object Reference") (OtherActor :type "Actor Object Reference") (OtherComp :type "PrimitiveComponent Object Reference") (OtherBodyIndex :type Integer) (bFromSweep :type Boolean) (SweepResult :type "HitResult Structure (by ref)"))
  (bind _asbp_learning_kit_player_character (cast `/Game/Edited_Assets/Actors/BP_LearningKit_PlayerCharacter` OtherActor))
  (bind _output_get (set `/Game/Edited_Assets/Actors/BP_LearningKit_PlayerCharacter.Current Health` (- (`/Game/Edited_Assets/Actors/BP_LearningKit_PlayerCharacter.Current Health` _asbp_learning_kit_player_character) 25.0) _asbp_learning_kit_player_character))
  (`/Game/Edited_Assets/UI/WB_HealthBar.UpdateHealthBar` (`/Game/Edited_Assets/Actors/BP_LearningKit_PlayerCharacter.WB Health Bar` _asbp_learning_kit_player_character) _output_get)
  (bind (_returnvalue_x _returnvalue_y) (`KismetMathLibrary.BreakVector` (`KismetMathLibrary.GetDirectionUnitVector` (`SceneComponent.K2_GetComponentLocation` (`self.Sphere`)) (`self.K2_GetActorLocation` _asbp_learning_kit_player_character))))
  (bind (_returnvalue_x_2 _returnvalue_y_2) (`KismetMathLibrary.BreakVector` (`KismetMathLibrary.Normal` (`KismetMathLibrary.MakeVector` _returnvalue_x _returnvalue_y))))
  (`Character.LaunchCharacter` _asbp_learning_kit_player_character (* (`KismetMathLibrary.MakeVector` _returnvalue_x_2 _returnvalue_y_2 1.0) (`self.LaunchVelocity`)) true true)
  (set `/Game/Edited_Assets/Actors/BP_LearningKit_PlayerCharacter.IsHit` true _asbp_learning_kit_player_character))

(fn `UserConstructionScript`)