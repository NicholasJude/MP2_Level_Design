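; Mortar projectile actor that explodes when its collision box overlaps the player or a static mesh actor.
; A player hit deducts health, updates the health bar, plays explosion effects, launches the player horizontally away from the capsule with upward lift and flags them as hit.
; A static mesh hit plays the same effects and spawns a short-lived BP_Explosion_Box at the impact point.
; Both cases destroy the projectile.
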(event `self.CollisionBox.OnComponentBeginOverlap`
  (params (OverlappedComponent :type "PrimitiveComponent Object Reference") (OtherActor :type "Actor Object Reference") (OtherComp :type "PrimitiveComponent Object Reference") (OtherBodyIndex :type Integer) (bFromSweep :type Boolean) (SweepResult :type "HitResult Structure (by ref)"))
  (bind _returnvalue (`self.K2_GetActorLocation`))
  (bind _returnvalue_2 (`self.K2_GetActorLocation`))
  (bind _asbp_learning_kit_player_character (cast `/Game/Edited_Assets/Actors/BP_LearningKit_PlayerCharacter` OtherActor)
    (:`then`
      (bind _output_get (set `/Game/Edited_Assets/Actors/BP_LearningKit_PlayerCharacter.Current Health` (- (`/Game/Edited_Assets/Actors/BP_LearningKit_PlayerCharacter.Current Health` _asbp_learning_kit_player_character) 25.0) _asbp_learning_kit_player_character))
      (`/Game/Edited_Assets/UI/WB_HealthBar.UpdateHealthBar` (`/Game/Edited_Assets/Actors/BP_LearningKit_PlayerCharacter.WB Health Bar` _asbp_learning_kit_player_character) _output_get)
      (`GameplayStatics.SpawnEmitterAtLocation` "/Game/StarterContent/Particles/P_Explosion.P_Explosion" _returnvalue_2)
      (`GameplayStatics.PlaySoundAtLocation` "/Game/StarterContent/Audio/Explosion_Cue.Explosion_Cue" _returnvalue_2 (struct) 1.0 1.0 0.0 null null null)
      (bind (_returnvalue_x _returnvalue_y) (`KismetMathLibrary.BreakVector` (`KismetMathLibrary.GetDirectionUnitVector` (`SceneComponent.K2_GetComponentLocation` (`self.CapsuleComponent`)) (`self.K2_GetActorLocation` _asbp_learning_kit_player_character))))
      (bind (_returnvalue_x_2 _returnvalue_y_2) (`KismetMathLibrary.BreakVector` (`KismetMathLibrary.Normal` (`KismetMathLibrary.MakeVector` _returnvalue_x _returnvalue_y))))
      (`self.LaunchCharacter` _asbp_learning_kit_player_character (* (`KismetMathLibrary.MakeVector` _returnvalue_x_2 _returnvalue_y_2 1.0) (`self.LaunchVelocity`)) false false)
      (set `/Game/Edited_Assets/Actors/BP_LearningKit_PlayerCharacter.IsHit` true _asbp_learning_kit_player_character)
      (`self.K2_DestroyActor`))
    (:`CastFailed`
      (cast `StaticMeshActor` OtherActor)
      (`GameplayStatics.SpawnEmitterAtLocation` "/Game/StarterContent/Particles/P_Explosion.P_Explosion" _returnvalue)
      (`GameplayStatics.PlaySoundAtLocation` "/Game/StarterContent/Audio/Explosion_Cue.Explosion_Cue" _returnvalue (struct) 1.0 1.0 0.0 null null null)
      (bind _output_get_2 (set `self.Explosion Location` _returnvalue))
      (`self.K2_DestroyActor`)
      (bind _returnvalue_3 (`|SpawnActorFromClass` "/Game/Edited_Assets/Actors/BP_Explosion_Box.BP_Explosion_Box_C" (`KismetMathLibrary.MakeTransform` _output_get_2) "Undefined" "OverrideRootScale" null null))
      (`self.SetLifeSpan` _returnvalue_3 0.2))))

(fn `UserConstructionScript`)