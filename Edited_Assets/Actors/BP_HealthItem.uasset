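; BP_HealthItem is a health pickup whose cube spins slowly around its vertical axis on Tick.
; When BP_LearningKit_PlayerCharacter overlaps the cube, it adds a fixed amount to CurrentHealth without clamping, unless health equals exactly 100.
; On pickup it refreshes the player's health bar widget, spawns an explosion particle and chime sound at its location, then destroys itself.
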(event `self.ReceiveTick`
  (params (DeltaSeconds :type "Float (single-precision)"))
  (`SceneComponent.K2_AddLocalRotation` (`self.Cube`) (`KismetMathLibrary.MakeRotator` 0.0 0.0 (* DeltaSeconds 30.0)) false false))

(event `self.Cube.OnComponentBeginOverlap`
  (params (OverlappedComponent :type "PrimitiveComponent Object Reference") (OtherActor :type "Actor Object Reference") (OtherComp :type "PrimitiveComponent Object Reference") (OtherBodyIndex :type Integer) (bFromSweep :type Boolean) (SweepResult :type "HitResult Structure (by ref)"))
  (bind _returnvalue (`self.K2_GetActorLocation`))
  (bind _asbp_learning_kit_player_character (cast `/Game/Edited_Assets/Actors/BP_LearningKit_PlayerCharacter` OtherActor))
  (bind _current_health (`/Game/Edited_Assets/Actors/BP_LearningKit_PlayerCharacter.Current Health` _asbp_learning_kit_player_character))
  (if (not (== _current_health 100.0))
    (bind _output_get (set `/Game/Edited_Assets/Actors/BP_LearningKit_PlayerCharacter.Current Health` (+ _current_health 25.0) _asbp_learning_kit_player_character))
    (`/Game/Edited_Assets/UI/WB_HealthBar.UpdateHealthBar` (`/Game/Edited_Assets/Actors/BP_LearningKit_PlayerCharacter.WB Health Bar` _asbp_learning_kit_player_character) _output_get)
    (`GameplayStatics.SpawnEmitterAtLocation` "/Game/StarterContent/Particles/P_Explosion.P_Explosion" _returnvalue)
    (`GameplayStatics.PlaySoundAtLocation` "/Game/LearningKit_Games/Assets/SFX/SFX_Chime_01A.SFX_Chime_01A" _returnvalue (struct) 1.0 1.0 0.0 null null null)
    (`self.K2_DestroyActor`)))

(fn `UserConstructionScript`)