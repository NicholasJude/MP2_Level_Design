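; BP_Level_Complete is a level-end trigger that finishes the level when the learning kit player character overlaps its Cube component.
; On overlap, it casts to BP_LearningKit_PlayerCharacter, adds that character's level-complete widget to the viewport, and switches to UI-only input with a visible cursor.
; It then moves the character away by a fixed Y and Z offset, sets its Complete flag, and hides it in game.
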(event `self.Cube.OnComponentBeginOverlap`
  (params (OverlappedComponent :type "PrimitiveComponent Object Reference") (OtherActor :type "Actor Object Reference") (OtherComp :type "PrimitiveComponent Object Reference") (OtherBodyIndex :type Integer) (bFromSweep :type Boolean) (SweepResult :type "HitResult Structure (by ref)"))
  (bind _returnvalue (`GameplayStatics.GetPlayerController` 0))
  (bind _asbp_learning_kit_player_character (cast `/Game/Edited_Assets/Actors/BP_LearningKit_PlayerCharacter` OtherActor))
  (`UserWidget.AddToViewport` (`/Game/Edited_Assets/Actors/BP_LearningKit_PlayerCharacter.WB Level Complete` _asbp_learning_kit_player_character) 0)
  (`WidgetBlueprintLibrary.SetInputMode_UIOnlyEx` _returnvalue null)
  (set `PlayerController.bShowMouseCursor` true _returnvalue)
  (bind (_returnvalue_x _returnvalue_y _returnvalue_z) (`KismetMathLibrary.BreakVector` (`self.K2_GetActorLocation` _asbp_learning_kit_player_character)))
  (`self.K2_SetActorLocation` _asbp_learning_kit_player_character (`KismetMathLibrary.MakeVector` _returnvalue_x (+ _returnvalue_y 1000.0) (+ _returnvalue_z 1500.0)) false false)
  (set `/Game/Edited_Assets/Actors/BP_LearningKit_PlayerCharacter.Complete` true _asbp_learning_kit_player_character)
  (`self.SetActorHiddenInGame` _asbp_learning_kit_player_character true))

(fn `UserConstructionScript`)